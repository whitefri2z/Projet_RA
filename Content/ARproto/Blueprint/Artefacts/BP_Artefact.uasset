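; BP_Artefact is a touchable artefact actor for the AR game that rewards score and reports its pickup to the interface.
; The construction script uses ArtefactID to choose its static mesh from the ArtefactsMesh array.
; Touching the mesh has BP_GameModeAR add difficulty-scaled score and raise the multiplier, then passes the ID to WidgetInterface as obtained.
; The actor does not hide or destroy itself here.
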(event `self.ArtefactMesh.OnInputTouchBegin`
  (params (FingerIndex :type "ETouchIndex Enum" :default "Touch1") (TouchedComponent :type "PrimitiveComponent Object Reference"))
  (bind _asbp_game_mode_ar (cast `/Game/ARproto/Blueprint/Gamemodes-States/BP_GameModeAR` (`GameplayStatics.GetGameMode`)))
  (`/Game/ARproto/Blueprint/Gamemodes-States/BP_GameModeAR.AddScore&Multiplier` _asbp_game_mode_ar (select `int` (`/Game/ARproto/Blueprint/Gamemodes-States/BP_GameModeAR.Difficulte` _asbp_game_mode_ar) :`0` 50 :`1` 100 :`2` 150) 1.0)
  (`/Game/ARproto/Widgets/Interface/WBP_Interface.ObtainedArtefact` (`/Game/ARproto/Blueprint/Gamemodes-States/BP_GameModeAR.Widget_Interface` _asbp_game_mode_ar) (`self.ArtefactID`)))

(fn `UserConstructionScript`
  (`StaticMeshComponent.SetStaticMesh` (`self.ArtefactMesh`) (`|GetArrayItem` (`self.ArtefactsMesh`) (`self.ArtefactID`))))