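; AR game mode that runs a timed score-attack round, starting the AR session, HUD and looping music.
; Tick counts down the round timer to the defeat screen, while EndGameWin, defined here, shows the victory screen.
; AddScoreMultiplier raises score and multiplier, restarts the multiplier decay window and grants bonus time at rising score thresholds.
; When that window expires, a resettable DoOnce drops the multiplier back to one.
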(event `self.ReceiveBeginPlay`
  (`ARBlueprintLibrary.StartARSession` "/Game/HandheldAR/D_ARSessionConfig.D_ARSessionConfig")
  (bind _returnvalue (`|CreateWidget` "/Game/ARproto/Widgets/Interface/WBP_Interface.WBP_Interface_C"))
  (bind _output_get (set `self.Widget_Interface` _returnvalue))
  (`UserWidget.AddToViewport` _output_get 0)
  (set `/Game/ARproto/Widgets/Interface/WBP_Interface.GameModeRef` self _output_get)
  (bind _returnvalue_2 (`GameplayStatics.SpawnSound2D` "/Game/Audio/Theme/Loop_Kings_Feast.Loop_Kings_Feast" 1.0 1.0 0.0 null))
  (set `self.CurrentMusic` _returnvalue_2))

(event `self.ReceiveTick`
  (params (DeltaSeconds :type "Float (single-precision)"))
  (if (`self.TimerIsRunning`)
    (`|ExecutionSequence`
      (:`then_0`
        (bind _output_get (set `self.Timer` (- (`self.Timer`) DeltaSeconds)))
        (bind _widget_interface (`self.Widget_Interface`)
          (:`then`
            (`/Game/ARproto/Widgets/Interface/WBP_Interface.TimerChanges` _widget_interface _output_get))
          (:`else`
            _))
        ;[1 1 1] Lose Condition
        (if (<= _output_get 0.0)
          (`/Engine/EditorBlueprintResources/StandardMacros.DoOnce` false
            (:`Completed`
              (bind _returnvalue (`|CreateWidget` "/Game/ARproto/Widgets/EndGame/WBP_EndGameDefeat.WBP_EndGameDefeat_C"))
              (`UserWidget.AddToViewport` _returnvalue 0)
              (set `self.TimerIsRunning` false)
              (`/Game/ARproto/Widgets/Interface/WBP_Interface.GameEnded` (`self.Widget_Interface`))
              (`AudioComponent.Stop` (`self.CurrentMusic`))))))
      (:`then_1`
        (if (> (`self.MultTimerBeforeReset`) 0.0)
          (bind _output_get_2 (set `self.MultTimerBeforeReset` (- (`self.MultTimerBeforeReset`) DeltaSeconds)))
          (`/Game/ARproto/Widgets/Interface/WBP_Interface.TimerForMultiplier` (`self.Widget_Interface`) false _output_get_2)
          (else
            (`/Engine/EditorBlueprintResources/StandardMacros.DoOnce` false :!label _label
              (:`Completed`
                (set `self.Multiplier` 1.0)
                (`/Game/ARproto/Widgets/Interface/WBP_Interface.TimerForMultiplier` (`self.Widget_Interface`) false 0.0)))))))))

(event `MultiplierCanGoDownAgain`
  (goto _label :!via `Reset`))

(fn `AddMultiplier`
  (params (MultiplierAddition :type "Float (double-precision)"))
  (set `self.Multiplier` (+ MultiplierAddition (`self.Multiplier`))))

(fn `AddScore`
  (params (ScoreAdded :type Integer))
  (set `self.Score` (+ (`self.Score`) (* (`KismetMathLibrary.FTrunc` (/ (* ScoreAdded (`self.Multiplier`)) 10.0)) 10)))
  (`/Game/ARproto/Widgets/Interface/WBP_Interface.Change Score And/ Or Mult` (`self.Widget_Interface`) (`self.Score`) ScoreAdded (`self.Multiplier`) 0.0 false))

(fn `AddScore&Multiplier`
  (params (ScoreAddition :type Integer) (MultiplierAddition :type "Float (double-precision)"))
  (set `self.Score` (+ (`self.Score`) (* (`KismetMathLibrary.FTrunc` (/ (* ScoreAddition (`self.Multiplier`)) 10.0)) 10)))
  (set `self.Multiplier` (+ (`self.Multiplier`) MultiplierAddition))
  (`/Game/ARproto/Widgets/Interface/WBP_Interface.Change Score And/ Or Mult` (`self.Widget_Interface`) (`self.Score`) ScoreAddition (`self.Multiplier`) MultiplierAddition true)
  (bind _output_get (set `self.MultTimerBeforeReset` 5.0))
  (`/Game/ARproto/Widgets/Interface/WBP_Interface.TimerForMultiplier` (`self.Widget_Interface`) true _output_get)
  (`self.MultiplierCanGoDownAgain`)
  (if (>= (`self.Score`) (`self.ScoreLimitForTimerAdd`))
    (set `self.ScoreLimitForTimerAdd` (+ (`self.ScoreLimitForTimerAdd`) 500))
    (set `self.Timer` (+ (`self.Timer`) 10.0))))

(fn `BreakChain`
  (params (ScoreLost :type Integer))
  (set `self.Multiplier` 1.0))

(fn `EndGameWin`
  (`/Game/ARproto/Widgets/Interface/WBP_Interface.GameEnded` (`self.Widget_Interface`))
  (bind _returnvalue (`|CreateWidget` "/Game/ARproto/Widgets/EndGame/WBP_EndGameWin.WBP_EndGameWin_C"))
  (`UserWidget.AddToViewport` _returnvalue 0)
  (set `self.TimerIsRunning` false)
  (`AudioComponent.Stop` (`self.CurrentMusic`)))

(fn `UserConstructionScript`)