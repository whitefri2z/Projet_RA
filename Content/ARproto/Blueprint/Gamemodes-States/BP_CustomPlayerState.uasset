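; Player state for the AR game mode that responds to artefact collection and triggers the win condition.
; On BeginPlay it caches a reference to BP_GameModeAR.
; When an artefact is collected, it notifies the game mode's widget interface, then ends the game as a win once the collected count reaches three.
; The count is only read here, not incremented.
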(event `self.ReceiveBeginPlay`
  (bind _asbp_game_mode_ar (cast `/Game/ARproto/Blueprint/Gamemodes-States/BP_GameModeAR` (`GameplayStatics.GetGameMode`)))
  (set `self.GameModeRef` _asbp_game_mode_ar))

(event `self.OnArtefactCollected`
  (`/Game/ARproto/Widgets/Interface/WBP_Interface.ObtainedArtefact` (`/Game/ARproto/Blueprint/Gamemodes-States/BP_GameModeAR.Widget_Interface` (`self.GameModeRef`)) 0)
  (if (>= (`self.GetArtefactsCollected`) 3)
    (`/Game/ARproto/Blueprint/Gamemodes-States/BP_GameModeAR.EndGameWin` (`self.GameModeRef`))))

(fn `UserConstructionScript`)