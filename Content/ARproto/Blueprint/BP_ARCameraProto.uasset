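; BP_ARCameraProto is a prototype AR camera actor that starts the AR session on BeginPlay and stops it on EndPlay.
; FocusonActor moves it to a given location via the GoToActor timeline, and ResetFocus reverses that move.
; FeedLightEstimate, not called here, applies AR ambient light intensity to the first directional light and skylight, plus color to the directional light.
; A projectile hit only prints "HIT".
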(event `self.ReceiveBeginPlay`
  (`ARBlueprintLibrary.StartARSession` "/Game/HandheldAR/D_ARSessionConfig.D_ARSessionConfig"))

(event `self.ReceiveEndPlay`
  (params (EndPlayReason :type "EEndPlayReason Enum" :default "Destroyed"))
  (`ARBlueprintLibrary.StopARSession`))

(event `self.ReceiveTick`
  (params (DeltaSeconds :type "Float (single-precision)"))
  (set `self.Delta Seconds` DeltaSeconds))

(event `InteractionInterface.ActorHitByProjectile`
  (`KismetSystemLibrary.PrintString` "HIT"))

(event `InteractionInterface.FocusOnActor`
  (params (FocusLocation :type "Vector Structure"))
  (set `self.TargetLocation` FocusLocation)
  (set `self.StartLocation` (`self.K2_GetActorLocation`))
  (bind (_direction _moveto) (`Timeline|GoToActor` :!via `PlayFromStart` :!label _label)
    (:`Update`
      (`self.K2_SetActorLocation` (`KismetMathLibrary.VLerp` (`self.StartLocation`) (`self.TargetLocation`) _moveto)))))

(event `ResetFocus`
  (goto _label :!via `ReverseFromEnd`))

(fn `FeedLightEstimate`
  (bind _asarbasic_light_estimate (cast `ARBasicLightEstimate` (`ARBlueprintLibrary.GetCurrentLightEstimate`)))
  (`|ExecutionSequence`
    (:`then_0`
      ;[1 1 1] Set directional light
      (bind _outactors (`GameplayStatics.GetAllActorsOfClass` "/Script/Engine.DirectionalLight"))
      (bind _output (`|GetArrayItem` _outactors))
      (`/Engine/EditorBlueprintResources/StandardMacros.IsValid` _output
        (:`Is Valid`
          (bind _lightcomponent (`Light.LightComponent` _output))
          (bind _returnvalue (/ (`ARBasicLightEstimate.GetAmbientIntensityLumens` _asarbasic_light_estimate) 1000.0))
          (`LightComponent.SetIntensity` _lightcomponent _returnvalue)
          (`LightComponent.SetLightColor` _lightcomponent (`ARBasicLightEstimate.GetAmbientColor` _asarbasic_light_estimate) true))))
    (:`then_1`
      ;[1 1 1] Set skylight
      (bind _outactors_2 (`GameplayStatics.GetAllActorsOfClass` "/Script/Engine.SkyLight"))
      (bind _output_2 (`|GetArrayItem` _outactors_2))
      (`/Engine/EditorBlueprintResources/StandardMacros.IsValid` _output_2
        (:`Is Valid`
          (`SkyLightComponent.SetIntensity` (`SkyLight.LightComponent` _output_2) _returnvalue))))))

(fn `UserConstructionScript`)