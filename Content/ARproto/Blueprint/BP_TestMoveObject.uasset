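; Test actor for dragging a cube by touch, moving it through the world while a finger is held after pressing on it.
; Touch begin on the cube stores the screen position of the first finger.
; Each Tick deprojects that start and the current position, nudging the cube a fixed step along the direction between them.
; Touch end or leave stops movement; an alternative line-trace placement routine is left unconnected.
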(event `self.ReceiveBeginPlay`
  (set `self.NewVar` (`GameplayStatics.GetPlayerController` 0)))

(event `self.ReceiveTick`
  (params (DeltaSeconds :type "Float (single-precision)"))
  (if (`self.IsTouch`)
    (bind _newvar (`self.NewVar`)
      (:`then`
        (bind (_locationx _locationy _biscurrentlypressed) (`PlayerController.GetInputTouchState` _newvar "Touch1"))
        (if _biscurrentlypressed
          (set `self.NewVar_0` (`KismetMathLibrary.MakeVector2D` _locationx _locationy))
          (`SceneComponent.K2_SetWorldLocation` (`self.Cube`) (+ (`SceneComponent.K2_GetComponentLocation` (`self.Cube`)) (* (`KismetMathLibrary.GetDirectionUnitVector` (`GameplayStatics.DeprojectScreenToWorld` (`self.NewVar`) (`self.NewVar_1`)) (`GameplayStatics.DeprojectScreenToWorld` (`self.NewVar`) (`self.NewVar_0`))) 0.3)) false false)
          (else
            (set `self.IsTouch` false))))
      (:`else`))))

(event `self.Cube.OnInputTouchBegin`
  (params (FingerIndex :type "ETouchIndex Enum" :default "Touch1") (TouchedComponent :type "PrimitiveComponent Object Reference"))
  (if (`|EnumEquality` FingerIndex "Touch1")
    (bind _newvar (`self.NewVar`)
      (:`then`
        (bind (_locationx _locationy) (`PlayerController.GetInputTouchState` _newvar "Touch1"))
        (set `self.NewVar_1` (`KismetMathLibrary.MakeVector2D` _locationx _locationy))
        (set `self.IsTouch` true))
      (:`else`))))

(event `self.Cube.OnInputTouchEnd`
  (params (FingerIndex :type "ETouchIndex Enum" :default "Touch1") (TouchedComponent :type "PrimitiveComponent Object Reference"))
  (`KismetSystemLibrary.PrintString` "Hello")
  (set `self.IsTouch` false))

(event `self.Cube.OnInputTouchLeave`
  (params (FingerIndex :type "ETouchIndex Enum" :default "Touch1") (TouchedComponent :type "PrimitiveComponent Object Reference"))
  (`KismetSystemLibrary.PrintString` "Hello")
  (set `self.IsTouch` false))

(fn `UserConstructionScript`)