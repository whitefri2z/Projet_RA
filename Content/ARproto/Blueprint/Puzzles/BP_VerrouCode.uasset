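; BP_VerrouCode is a touch-driven combination lock puzzle with three rotatable cylinders, apparently unfinished.
; Touching a cylinder with the first finger stores it and the start position, enabling rotation until release.
; Tick deprojects start and current touch points, adding their negated X direction to the cylinder's pitch reading, applied as roll.
; A looping timer calls TestValueCode, which is empty, so no code is checked; digit-conversion debug prints are disconnected.
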(event `self.ReceiveBeginPlay`
  (set `self.Player controller` (`GameplayStatics.GetPlayerController` 0))
  (`KismetSystemLibrary.K2_SetTimerDelegate` (delegate `TestValueCode`) 0.5 true)
  (`SceneComponent.K2_SetWorldRotation` (`self.Cylinder`) (struct :`Pitch` 180.0 :`Roll` 90.0) false false))

(event `TestValueCode`)

(event `self.ReceiveTick`
  (params (DeltaSeconds :type "Float (single-precision)"))
  (bind _refrotatecylindre (`self.RefRotateCylindre`))
  (bind (_returnvalue_roll _returnvalue_pitch) (`KismetMathLibrary.BreakRotator` (`SceneComponent.K2_GetComponentRotation` _refrotatecylindre)))
  (if (`self.CanRotate`)
    (bind _player_controller (`self.Player controller`)
      (:`then`
        (bind (_locationx _locationy _biscurrentlypressed) (`PlayerController.GetInputTouchState` _player_controller "Touch1"))
        (if _biscurrentlypressed
          (set `self.NewPosition` (`KismetMathLibrary.MakeVector2D` _locationx _locationy))
          (`SceneComponent.K2_SetWorldRotation` _refrotatecylindre (`KismetMathLibrary.MakeRotator` (+ _returnvalue_pitch (* (.x (`KismetMathLibrary.GetDirectionUnitVector` (`GameplayStatics.DeprojectScreenToWorld` (`self.Player controller`) (`self.StartPosition`)) (`GameplayStatics.DeprojectScreenToWorld` (`self.Player controller`) (`self.NewPosition`)))) -1.0))) false false)
          (else
            (set `self.CanRotate` false))))
      (:`else`))))

(event `self.Cylinder1.OnInputTouchBegin`
  (params (FingerIndex :type "ETouchIndex Enum" :default "Touch1") (TouchedComponent :type "PrimitiveComponent Object Reference"))
  (bind _returnvalue (`|EnumEquality` FingerIndex "Touch1"))
  (if _returnvalue
    (set `self.CanRotate` _returnvalue)
    (bind _player_controller (`self.Player controller`)
      (:`then`
        (bind (_locationx _locationy) (`PlayerController.GetInputTouchState` _player_controller "Touch1"))
        (set `self.StartPosition` (`KismetMathLibrary.MakeVector2D` _locationx _locationy))
        (set `self.RefRotateCylindre` (`self.Cylinder1`)))
      (:`else`))))

(event `self.Cylinder2.OnInputTouchBegin`
  (params (FingerIndex :type "ETouchIndex Enum" :default "Touch1") (TouchedComponent :type "PrimitiveComponent Object Reference"))
  (bind _returnvalue (`|EnumEquality` FingerIndex "Touch1"))
  (if _returnvalue
    (set `self.CanRotate` _returnvalue)
    (bind _player_controller (`self.Player controller`)
      (:`then`
        (bind (_locationx _locationy) (`PlayerController.GetInputTouchState` _player_controller "Touch1"))
        (set `self.StartPosition` (`KismetMathLibrary.MakeVector2D` _locationx _locationy))
        (set `self.RefRotateCylindre` (`self.Cylinder2`)))
      (:`else`))))

(event `self.Cylinder.OnInputTouchBegin`
  (params (FingerIndex :type "ETouchIndex Enum" :default "Touch1") (TouchedComponent :type "PrimitiveComponent Object Reference"))
  (bind _returnvalue (`|EnumEquality` FingerIndex "Touch1"))
  (if _returnvalue
    (set `self.CanRotate` _returnvalue)
    (bind _player_controller (`self.Player controller`)
      (:`then`
        (bind (_locationx _locationy) (`PlayerController.GetInputTouchState` _player_controller "Touch1"))
        (set `self.StartPosition` (`KismetMathLibrary.MakeVector2D` _locationx _locationy))
        (set `self.RefRotateCylindre` (`self.Cylinder`)))
      (:`else`))))

(fn `UserConstructionScript`)