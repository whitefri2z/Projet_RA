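; BP_CubeInteractWithFace is an AR puzzle cube actor that colours a face and plays puzzle feedback sounds.
; SetFaceColor creates a dynamic material instance on CubeMesh and passes it the face normal and colour as parameters, then plays a glow sound.
; SuccessPuzzel plays the artefact-gain sound.
; The touch handler on the mesh is empty, and nothing in this Blueprint calls either custom event.
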(event `self.CubeMesh.OnInputTouchBegin`
  (params (FingerIndex :type "ETouchIndex Enum" :default "Touch1") (TouchedComponent :type "PrimitiveComponent Object Reference")))

(event `self.SetFaceColor`
  (params (NormalFace :type "Vector Structure") (Color :type "LinearColor Structure"))
  (bind _cubemesh (`self.CubeMesh`))
  (bind _returnvalue (`PrimitiveComponent.CreateDynamicMaterialInstance` _cubemesh 0 (`PrimitiveComponent.GetMaterial` _cubemesh 0) "None"))
  (bind _output_get (set `self.Dynamic Material Instace` _returnvalue))
  (`MaterialInstanceDynamic.SetScalarParameterValue` _output_get "ParamX" (.x NormalFace))
  (`MaterialInstanceDynamic.SetScalarParameterValue` _output_get "ParamY" (.y NormalFace))
  (`MaterialInstanceDynamic.SetScalarParameterValue` _output_get "ParamZ" (.z NormalFace))
  (`MaterialInstanceDynamic.SetVectorParameterValue` _output_get "ColorFace" Color)
  (`GameplayStatics.PlaySound2D` "/Game/Audio/Dice/GlowingFace.GlowingFace" 1.0 1.0 0.0 null null))

(event `InteractionInterface.SuccessPuzzel`
  (`GameplayStatics.PlaySound2D` "/Game/Audio/Win-Loose/GainArtefact.GainArtefact" 1.0 1.0 0.0 null null))

(fn `UserConstructionScript`)