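; BP_Padlock is a touch-operated numeric padlock puzzle actor with a text display and ten keyhole components numbered 0 to 9.
; Touching any keyhole only plays the SwapNumber sound; digit entry and code checking are absent, and the mesh touch event is empty.
; EffectErreur uses delays to flash the text between "XXX" and the current code, then resets the display and CodePadlockString to "___".
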(event `self.EffectErreur`
  (`TextRenderComponent.K2_SetText` (`self.PadlockText`) "XXX")
  (`KismetSystemLibrary.Delay` 0.5)
  (`TextRenderComponent.K2_SetText` (`self.PadlockText`) (`KismetTextLibrary.Conv_StringToText` (`self.CodePadlockString`)))
  (`KismetSystemLibrary.Delay` 0.5)
  (`TextRenderComponent.K2_SetText` (`self.PadlockText`) "XXX")
  (`KismetSystemLibrary.Delay` 0.5)
  (`TextRenderComponent.K2_SetText` (`self.PadlockText`) (`KismetTextLibrary.Conv_StringToText` (`self.CodePadlockString`)))
  (`KismetSystemLibrary.Delay` 0.5)
  (`TextRenderComponent.K2_SetText` (`self.PadlockText`) "XXX")
  (`KismetSystemLibrary.Delay` 0.5)
  (`TextRenderComponent.K2_SetText` (`self.PadlockText`) "___")
  (set `self.CodePadlockString` "___"))

(event `self.PadlockMesh.OnInputTouchBegin`
  (params (FingerIndex :type "ETouchIndex Enum" :default "Touch1") (TouchedComponent :type "PrimitiveComponent Object Reference")))

(event `self.PadlockKeyhole1.OnInputTouchBegin`
  (params (FingerIndex :type "ETouchIndex Enum" :default "Touch1") (TouchedComponent :type "PrimitiveComponent Object Reference"))
  (`GameplayStatics.PlaySound2D` "/Game/Audio/Code/SwapNumber.SwapNumber" 1.0 1.0 0.0 null null))

(event `self.PadlockKeyhole2.OnInputTouchBegin`
  (params (FingerIndex :type "ETouchIndex Enum" :default "Touch1") (TouchedComponent :type "PrimitiveComponent Object Reference"))
  (`GameplayStatics.PlaySound2D` "/Game/Audio/Code/SwapNumber.SwapNumber" 1.0 1.0 0.0 null null))

(event `self.PadlockKeyhole3.OnInputTouchBegin`
  (params (FingerIndex :type "ETouchIndex Enum" :default "Touch1") (TouchedComponent :type "PrimitiveComponent Object Reference"))
  (`GameplayStatics.PlaySound2D` "/Game/Audio/Code/SwapNumber.SwapNumber" 1.0 1.0 0.0 null null))

(event `self.PadlockKeyhole0.OnInputTouchBegin`
  (params (FingerIndex :type "ETouchIndex Enum" :default "Touch1") (TouchedComponent :type "PrimitiveComponent Object Reference"))
  (`GameplayStatics.PlaySound2D` "/Game/Audio/Code/SwapNumber.SwapNumber" 1.0 1.0 0.0 null null))

(event `self.PadlockKeyhole9.OnInputTouchBegin`
  (params (FingerIndex :type "ETouchIndex Enum" :default "Touch1") (TouchedComponent :type "PrimitiveComponent Object Reference"))
  (`GameplayStatics.PlaySound2D` "/Game/Audio/Code/SwapNumber.SwapNumber" 1.0 1.0 0.0 null null))

(event `self.PadlockKeyhole8.OnInputTouchBegin`
  (params (FingerIndex :type "ETouchIndex Enum" :default "Touch1") (TouchedComponent :type "PrimitiveComponent Object Reference"))
  (`GameplayStatics.PlaySound2D` "/Game/Audio/Code/SwapNumber.SwapNumber" 1.0 1.0 0.0 null null))

(event `self.PadlockKeyhole7.OnInputTouchBegin`
  (params (FingerIndex :type "ETouchIndex Enum" :default "Touch1") (TouchedComponent :type "PrimitiveComponent Object Reference"))
  (`GameplayStatics.PlaySound2D` "/Game/Audio/Code/SwapNumber.SwapNumber" 1.0 1.0 0.0 null null))

(event `self.PadlockKeyhole5.OnInputTouchBegin`
  (params (FingerIndex :type "ETouchIndex Enum" :default "Touch1") (TouchedComponent :type "PrimitiveComponent Object Reference"))
  (`GameplayStatics.PlaySound2D` "/Game/Audio/Code/SwapNumber.SwapNumber" 1.0 1.0 0.0 null null))

(event `self.PadlockKeyhole6.OnInputTouchBegin`
  (params (FingerIndex :type "ETouchIndex Enum" :default "Touch1") (TouchedComponent :type "PrimitiveComponent Object Reference"))
  (`GameplayStatics.PlaySound2D` "/Game/Audio/Code/SwapNumber.SwapNumber" 1.0 1.0 0.0 null null))

(event `self.PadlockKeyhole4.OnInputTouchBegin`
  (params (FingerIndex :type "ETouchIndex Enum" :default "Touch1") (TouchedComponent :type "PrimitiveComponent Object Reference"))
  (`GameplayStatics.PlaySound2D` "/Game/Audio/Code/SwapNumber.SwapNumber" 1.0 1.0 0.0 null null))

(fn `UserConstructionScript`)