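; Simon puzzle actor with four button meshes, providing timed color flashes for one button or all of them.
; ColorButton picks a mesh by step index, tints the BaseColor of its dynamic material, then restores it after a half-second delay.
; ColorAllButtons tints all four and restores each to the last color read, using an instance array that is never cleared.
; Touch handlers are empty and no sequence logic is present.
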(event `self.ColorButton`
  (params (StepIndex :type Integer) (ButtonColor :type "LinearColor Structure"))
  (bind _returnvalue (select `int` StepIndex :`0` (`self.SimonButtonMesh1`) :`1` (`self.SimonButtonMesh2`) :`2` (`self.SimonButtonMesh3`) :`3` (`self.SimonButtonMesh4`)))
  (bind _returnvalue_2 (`PrimitiveComponent.CreateDynamicMaterialInstance` _returnvalue 0 (`PrimitiveComponent.GetMaterial` _returnvalue 0) "None"))
  (bind _output_get (set `self.DynamicMaterialInstance` _returnvalue_2))
  (bind _returnvalue_3 (`MaterialInstanceDynamic.K2_GetVectorParameterValue` _output_get "BaseColor"))
  (set `self.BaseColor` _returnvalue_3)
  (`MaterialInstanceDynamic.SetVectorParameterValue` _output_get "BaseColor" ButtonColor)
  (`KismetSystemLibrary.Delay` 0.5)
  (`MaterialInstanceDynamic.SetVectorParameterValue` (`self.DynamicMaterialInstance`) "BaseColor" (`self.BaseColor`)))

(event `self.ColorAllButtons`
  (params (ButtonColor :type "LinearColor Structure"))
  (for _array_element (`|MakeArray` (`self.SimonButtonMesh1`) (`self.SimonButtonMesh2`) (`self.SimonButtonMesh3`) (`self.SimonButtonMesh4`))
    (bind _returnvalue (`PrimitiveComponent.CreateDynamicMaterialInstance` _array_element 0 (`PrimitiveComponent.GetMaterial` _array_element 0) "None"))
    (bind _returnvalue_2 (`MaterialInstanceDynamic.K2_GetVectorParameterValue` _returnvalue "BaseColor"))
    (set `self.BaseColor` _returnvalue_2)
    (`KismetArrayLibrary.Array_Add` (`self.ArrayDynamicMaterialInstance`) _returnvalue)
    (`MaterialInstanceDynamic.SetVectorParameterValue` _returnvalue "BaseColor" ButtonColor))
  (`KismetSystemLibrary.Delay` 0.5)
  (for _array_element_2 (`self.ArrayDynamicMaterialInstance`)
    (`MaterialInstanceDynamic.SetVectorParameterValue` _array_element_2 "BaseColor" (`self.BaseColor`))))

(event `self.SimonButtonMesh1.OnInputTouchBegin`
  (params (FingerIndex :type "ETouchIndex Enum" :default "Touch1") (TouchedComponent :type "PrimitiveComponent Object Reference")))

(event `self.SimonButtonMesh2.OnInputTouchBegin`
  (params (FingerIndex :type "ETouchIndex Enum" :default "Touch1") (TouchedComponent :type "PrimitiveComponent Object Reference")))

(event `self.SimonButtonMesh3.OnInputTouchBegin`
  (params (FingerIndex :type "ETouchIndex Enum" :default "Touch1") (TouchedComponent :type "PrimitiveComponent Object Reference")))

(event `self.SimonButtonMesh4.OnInputTouchBegin`
  (params (FingerIndex :type "ETouchIndex Enum" :default "Touch1") (TouchedComponent :type "PrimitiveComponent Object Reference")))

(event `self.SimonMesh.OnInputTouchBegin`
  (params (FingerIndex :type "ETouchIndex Enum" :default "Touch1") (TouchedComponent :type "PrimitiveComponent Object Reference")))

(fn `UserConstructionScript`)